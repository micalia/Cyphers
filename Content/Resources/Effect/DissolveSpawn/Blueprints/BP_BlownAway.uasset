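; BP_BlownAway is an effect actor that loops a visibility sweep on a skeletal mesh alongside a Niagara effect.
; Each Tick writes a falling VisibilityLevel to the mesh materials and MPC_Global, using a fixed per-frame step that is frame-rate dependent.
; Below a threshold it deactivates Niagara, then a DoOnce-gated delay resets the level and reactivates Niagara.
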(event `self.ReceiveBeginPlay`)

(event `self.ReceiveTick`
  (params (DeltaSeconds :type "Float (single-precision)"))
  (bind _parameter_value (`self.Parameter Value`))
  (`MeshComponent.SetScalarParameterValueOnMaterials` (`self.SkeletalMesh`) "VisibilityLevel" _parameter_value)
  (`KismetMaterialLibrary.SetScalarParameterValue` "/Game/Resources/Effect/DissolveSpawn/Materials/Parametercollection/MPC_Global.MPC_Global" "VisibilityLevel" _parameter_value)
  (bind _output_get (set `self.Parameter Value` (- _parameter_value 0.5)))
  (if (< _output_get -20.0)
    (`ActorComponent.Deactivate` (`self.Niagara`))
    (`/Engine/EditorBlueprintResources/StandardMacros.DoOnce` false :!label _label
      (:`Completed`
        (`KismetSystemLibrary.Delay` 1.0)
        (set `self.Parameter Value` 400.0)
        (`ActorComponent.Activate` (`self.Niagara`) false)))
    (else
      (goto _label :!via `Reset`))))

(fn `UserConstructionScript`)