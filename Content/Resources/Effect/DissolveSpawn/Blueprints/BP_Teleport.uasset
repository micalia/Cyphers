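; BP_Teleport is a looping teleport dissolve effect on a skeletal mesh.
; On BeginPlay it derives top, center and bottom points from the mesh bounds and creates a dynamic material instance.
; Two timelines alternate with one-second pauses, each driving the "Amount" material parameter while moving two static meshes between those ends and the center.
; The NSPortal effects activate for each timeline pass and deactivate when it finishes.
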(event `self.ReceiveBeginPlay`
  (bind _ns_portal (`self.NS_Portal`))
  (bind _skeletalmesh (`self.SkeletalMesh`))
  (bind _returnvalue (`SceneComponent.K2_GetComponentLocation` _skeletalmesh))
  (bind _z (.z (`.BoxExtent` (`KismetSystemLibrary.GetComponentBounds` _skeletalmesh))))
  (set `self.upperStartLoc` (+ _returnvalue (`KismetMathLibrary.MakeVector` 0.0 0.0 (* _z 2.0))))
  (set `self.CenterLocation` (+ _returnvalue (`KismetMathLibrary.MakeVector` 0.0 0.0 _z)))
  (set `self.lowerStartLoc` _returnvalue)
  (bind _returnvalue_2 (`PrimitiveComponent.CreateDynamicMaterialInstance` (`self.SkeletalMesh`) 0 null "None"))
  (set `self.DM` _returnvalue_2)
  (`ActorComponent.Activate` (`self.NS_Portal`) true :!label _label)
  (`ActorComponent.Activate` (`self.NS_Portal1`) true)
  (bind (_direction _newtrack_0) (`Timeline|Timeline_0` :!via `PlayFromStart`)
    (:`Update`
      (`MeshComponent.SetScalarParameterValueOnMaterials` (`self.SkeletalMesh`) "Amount" (`KismetMathLibrary.Lerp` -4.0 0.5 _newtrack_0))
      (`SceneComponent.K2_SetWorldLocation` (`self.StaticMesh`) (`KismetMathLibrary.VLerp` (`self.upperStartLoc`) (`self.CenterLocation`) _newtrack_0) false false)
      (`SceneComponent.K2_SetWorldLocation` (`self.StaticMesh1`) (`KismetMathLibrary.VLerp` (`self.lowerStartLoc`) (`self.CenterLocation`) _newtrack_0) false false))
    (:`Finished`
      (`ActorComponent.Deactivate` _ns_portal)
      (`ActorComponent.Deactivate` (`self.NS_Portal1`))
      (`KismetSystemLibrary.Delay` 1.0)
      (`ActorComponent.Activate` _ns_portal true)
      (`ActorComponent.Activate` (`self.NS_Portal1`) true)
      (bind (_direction_2 _newtrack_0_2) (`Timeline|Timeline_1` :!via `PlayFromStart`)
        (:`Update`
          (`MeshComponent.SetScalarParameterValueOnMaterials` (`self.SkeletalMesh`) "Amount" (`KismetMathLibrary.Lerp` -4.0 0.5 _newtrack_0_2))
          (`SceneComponent.K2_SetWorldLocation` (`self.StaticMesh`) (`KismetMathLibrary.VLerp` (`self.upperStartLoc`) (`self.CenterLocation`) _newtrack_0_2) false false)
          (`SceneComponent.K2_SetWorldLocation` (`self.StaticMesh1`) (`KismetMathLibrary.VLerp` (`self.lowerStartLoc`) (`self.CenterLocation`) _newtrack_0_2) false false))
        (:`Finished`
          (`ActorComponent.Deactivate` (`self.NS_Portal`))
          (`ActorComponent.Deactivate` (`self.NS_Portal1`))
          (`KismetSystemLibrary.Delay` 1.0)
          (goto _label))))))

(fn `UserConstructionScript`)