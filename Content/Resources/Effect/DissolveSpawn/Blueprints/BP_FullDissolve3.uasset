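; BP_FullDissolve3 is an actor that continuously dissolves and restores its skeletal mesh.
; A single timeline drives the Amount scalar parameter on the mesh's materials, playing from the start to disintegrate and reversing from the end to reintegrate.
; StartEffect runs on BeginPlay, alternates the two phases with fixed delays, then calls itself to loop indefinitely.
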(event `self.ReceiveBeginPlay`
  (`self.StartEffect`))

(event `DisIntegration`
  (bind (_direction _newtrack_0) (`Timeline|Timeline_0` :!via `PlayFromStart` :!label _label)
    (:`Update`
      (`MeshComponent.SetScalarParameterValueOnMaterials` (`self.SkeletalMesh`) "Amount" _newtrack_0))))

(event `ReIntegration`
  (goto _label :!via `ReverseFromEnd`))

(event `StartEffect`
  (`self.DisIntegration`)
  (`KismetSystemLibrary.Delay` 5.0)
  (`self.ReIntegration`)
  (`KismetSystemLibrary.Delay` 5.0)
  (`self.StartEffect`))

(fn `UserConstructionScript`)