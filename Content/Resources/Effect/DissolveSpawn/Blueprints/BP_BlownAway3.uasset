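; BP_BlownAway3 is a looping dissolve effect on a skeletal mesh, paired with a Niagara particle system.
; Starting on BeginPlay, Dissolve waits briefly, activates Niagara and plays a timeline that lerps the "Amount" scalar parameter on the mesh materials.
; When the timeline finishes, it deactivates Niagara, waits again and calls Dissolve, repeating the cycle indefinitely.
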(event `self.ReceiveBeginPlay`
  (`self.Dissolve`))

(event `Dissolve`
  (`KismetSystemLibrary.Delay` 1.0)
  (`ActorComponent.Activate` (`self.Niagara`) true)
  (bind (_direction _newtrack_0) (`Timeline|Timeline_0` :!via `PlayFromStart`)
    (:`Update`
      (`MeshComponent.SetScalarParameterValueOnMaterials` (`self.SkeletalMesh`) "Amount" (`KismetMathLibrary.Lerp` -4.0 0.5 _newtrack_0)))
    (:`Finished`
      (`ActorComponent.Deactivate` (`self.Niagara`))
      (`KismetSystemLibrary.Delay` 1.0)
      (`self.Dissolve`))))

(fn `UserConstructionScript`)